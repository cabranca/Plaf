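; GA_Punch is a Gameplay Ability that performs a punch attack.
; On activation it commits, starts the AM_attack montage, and immediately applies GE_Recover_Stamina to the owner with a SetByCaller magnitude of zero.
; It waits once for the Event.Montage.Punch gameplay event and applies GE_Punch to the target data in its payload.
; Every montage exit prints a debug string and ends the ability.
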(event `self.K2_ActivateAbility`
  (`self.K2_CommitAbility`)
  (`AbilityTask_PlayMontageAndWait.CreatePlayMontageAndWaitProxy` "None" "/Game/ElfArden/Animations/AM_attack.AM_attack" 1.0 "None" false
    (:`then`
      (bind _returnvalue (`AbilitySystemBlueprintLibrary.AssignTagSetByCallerMagnitude` (`self.MakeOutgoingGameplayEffectSpec` "/Game/Blueprints/GAS/Effects/GE_Recover_Stamina.GE_Recover_Stamina_C") (struct) 0.0))
      (`self.K2_ApplyGameplayEffectSpecToOwner` _returnvalue)
      (bind (_asynctaskproxy _payload) (`AbilityTask_WaitGameplayEvent.WaitGameplayEvent` (struct :`TagName` "Event.Montage.Punch") null true)
        (:`EventReceived`
          (`self.BP_ApplyGameplayEffectToTarget` (`.TargetData` (break `GameplayEventData` _payload)) "/Game/Blueprints/GAS/Effects/GE_Punch.GE_Punch_C"))))
    (:`OnCompleted`
      (`KismetSystemLibrary.PrintString` "On Completed")
      (`self.K2_EndAbility` :!label _label))
    (:`OnBlendOut`
      (`KismetSystemLibrary.PrintString` "On Blend Out")
      (goto _label))
    (:`OnInterrupted`
      (`KismetSystemLibrary.PrintString` "On Interrupted")
      (goto _label))
    (:`OnCancelled`
      (`KismetSystemLibrary.PrintString` "On Cancelled")
      (goto _label))))