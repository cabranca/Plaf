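; BP_MainCharacter is the player character Blueprint, providing a melee punch through the Gameplay Ability System.
; On BeginPlay it snaps FistCollider to the mesh's left-hand socket, and the basic attack input activates GA_Punch.
; When the fist overlaps another actor, the character sends itself an Event.Montage.Punch gameplay event carrying that actor as target data, leaving hit handling outside this Blueprint.
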(event `self.ReceiveBeginPlay`
  (`SceneComponent.K2_AttachToComponent` (`self.Fist Collider`) (`self.Mesh`) "hand_l" "SnapToTarget" "KeepRelative" "KeepRelative" true))

(event `EnhancedInput|/Game/Input/IA_BasicAttack`
  (params (ActionValue :type Boolean) (ElapsedSeconds :type "Float (double-precision)") (TriggeredSeconds :type "Float (double-precision)") (InputAction :type "InputAction Object Reference" :default "/Game/Input/IA_BasicAttack.IA_BasicAttack"))
  (:`Triggered`
    (`AbilitySystemComponent.TryActivateAbilityByClass` (`AbilitySystemBlueprintLibrary.GetAbilitySystemComponent` null) "/Game/Blueprints/GAS/Punch/GA_Punch.GA_Punch_C" true)))

(event `self.Fist Collider.OnComponentBeginOverlap`
  (params (OverlappedComponent :type "PrimitiveComponent Object Reference") (OtherActor :type "Actor Object Reference") (OtherComp :type "PrimitiveComponent Object Reference") (OtherBodyIndex :type Integer) (bFromSweep :type Boolean) (SweepResult :type "HitResult Structure (by ref)"))
  (if (!= OtherActor self)
    (`AbilitySystemBlueprintLibrary.SendGameplayEventToActor` self (struct :`TagName` "Event.Montage.Punch") (make `GameplayEventData` (struct) self OtherActor null null (struct) (struct) (struct) 0.0 (`AbilitySystemBlueprintLibrary.AbilityTargetDataFromActor` OtherActor)))))

(fn `UserConstructionScript`)